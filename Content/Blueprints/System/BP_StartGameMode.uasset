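; Game mode for the start screen that creates local players, shows the start window and plays background music.
; The first select press plays the window's button and bubble animations with a sound, then enables player input after a short delay.
; Tick polls each start controller's ready flag and disables input once all are ready, with debug mode checking only the first player.
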(event EventBeginPlay
  (CallFunction|Init)
  (Default|PlayBackGroundMusic (CallFunction|GetSoundManager) true "NewEnumerator1"))

(event EventTick
  (params (DeltaSeconds :type Float%20%28single-precision%29))
  (bind _isallready (CallFunction|IsReadyPlayers))
  (if _isallready
    (Variables|Default|SetCanPlayerInput false)))

(event EventInputSelectButton
  (params (InPlayerIndex :type Integer))
  (bind _startwindowwidget (Variables|Default|GetStartWindowWidget))
  (Utilities|FlowControl|DoOnce false
    (:Completed
      (Default|InputButton _startwindowwidget)
      (Default|PlayBubbleAnimation _startwindowwidget)
      (Default|PlaySoundEffect (CallFunction|GetSoundManager) "NewEnumerator0" "0, 0, 0")
      (Utilities|FlowControl|Delay 1.5)
      (Variables|Default|SetCanPlayerInput true))))

(fn ConstructionScript)

(fn Init
  (Utilities|FlowControl|Sequence
    (:then_0
      (for _index (range 0 3)
        (Class|GameplayStatics|CreatePlayer _index)
        (Default|Init (.AsBP%20Start%20Player%20Pawn (Utilities|Casting|CastToBP_StartPlayerPawn (Game|Player|GetPlayerPawn _index))))))
    (:then_1
      (bind _returnvalue (UserInterface|CreateWidget "/Game/Blueprints/Widget/BP_StartWindowWidget.BP_StartWindowWidget_C"))
      (bind _output_get (Variables|Default|SetStartWindowWidget _returnvalue))
      (UserInterface|Viewport|AddtoViewport _output_get 0)
      (Variables|Default|SetCanPlayerInput false))))

(fn IsReadyPlayers
  (for _index (range 0 3)
    (bind _output_get (LocalVariables|SetIsReady (and (Variables|/Game/Blueprints/Player/BP_StartPlayerController.BP_StartPlayerController_C|GetIsReady (.AsBP%20Start%20Player%20Controller (Utilities|Casting|CastToBP_StartPlayerController (Game|GetPlayerController _index)))) (LocalVariables|GetIsReady))))
    (bind _isdebug (Class|BPGameInstanceInterface|IsDebugMode(Message) (Game|GetGameInstance)))
    (if _isdebug
      (return _output_get)))
  (return (LocalVariables|GetIsReady)))
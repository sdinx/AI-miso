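; BP_SoundManager plays sound effects and background music looked up by enum name in a sound data table, which supplies asset and volume.
; Effects play at the given location, or as 2D sound when the location is zero.
; Music is stored as a persistent 2D component, started with optional fade-in and a bound finished event.
; StopBGM fades it out, or stops it instantly when passed -1, then clears the reference.
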(event EventBeginPlay)

(event Collision|EventActorBeginOverlap
  (params (OtherActor :type Actor%20Object%20Reference)))

(event EventTick
  (params (DeltaSeconds :type Float%20%28single-precision%29)))

(fn ConstructionScript)

(fn PlaySoundEffect
  (params (InSoundName :type ESoundName%20Enum :default "NewEnumerator4") (InEffectLocation :type Vector))
  (bind _returnvalue (Utilities|GetDataTableRow "/Game/Blueprints/Data/SoundDataTable.SoundDataTable" (Utilities|String|StringToName (Utilities|String|EnumtoString InSoundName)))
    (:then
      (if (Math|Vector|NotEqual(Vector) InEffectLocation "0, 0, 0" 0.0001)
        (Audio|PlaySoundatLocation (.SoundObject (Utilities|Struct|BreakStructSoundData _returnvalue)) InEffectLocation "0, 0, 0" (.Volume (Utilities|Struct|BreakStructSoundData _returnvalue)) 1.0 0.0 0 0 0)
        (else
          (Audio|PlaySound2D (.SoundObject (Utilities|Struct|BreakStructSoundData _returnvalue)) (.Volume (Utilities|Struct|BreakStructSoundData _returnvalue)) 1.0 0.0 0 0))))))

(fn PlayBackGroundMusic
  (params (IsFadeIn :type Boolean) (InSoundName :type ESoundName%20Enum :default "NewEnumerator4"))
  (Variables|Default|SetIsBGMFadeIn IsFadeIn)
  (bind _returnvalue (Utilities|GetDataTableRow "/Game/Blueprints/Data/SoundDataTable.SoundDataTable" (Utilities|String|StringToName (Utilities|String|EnumtoString InSoundName)))
    (:then
      (bind _returnvalue_2 (Audio|CreateSound2D (.SoundObject (Utilities|Struct|BreakStructSoundData _returnvalue)) (.Volume (Utilities|Struct|BreakStructSoundData _returnvalue)) 1.0 0.0 0 false false))
      (Variables|Default|SetCurrentBGM _returnvalue_2)
      (CallFunction|StartBGM))))

(fn StartBGM
  (bind _currentbgm (Variables|Default|GetCurrentBGM)
    (:then
      (if (Variables|Default|GetIsBGMFadeIn)
        (Audio|Components|Audio|FadeIn _currentbgm 2.0 1.0 0.0 :!class /Script/Engine.AudioComponent)
        (else
          (Audio|Components|Audio|Play _currentbgm 0.0)))
      (EventDispatchers|BindEventtoOnAudioFinished _currentbgm (EventDispatchers|CreateEvent :!event StartBGM)))
    (:else)))

(fn StopBGM
  (params (InFadeOutTime :type Float%20%28single-precision%29))
  (bind _currentbgm (Variables|Default|GetCurrentBGM)
    (:then
      (if (Math|Float|NearlyEqual(Float) InFadeOutTime -1.0 0.001)
        (Audio|Components|Audio|Stop _currentbgm)
        (else
          (Audio|Components|Audio|FadeOut _currentbgm InFadeOutTime 0.0 :!class /Script/Engine.AudioComponent)))
      (Variables|Default|SetCurrentBGM 0))
    (:else)))
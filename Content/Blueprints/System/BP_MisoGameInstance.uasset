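; Game instance that holds the game's active states in a set and exposes a debug-mode flag.
; Init seeds a default state, and interface events add, remove or clear states, with single adds optionally clearing the others first.
; Queries test one state or several combined by AND, OR or XOR, though the XOR branch only reflects the last state checked.
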(event EventInit
  (CallFunction|AddGameState "NewEnumerator0" false))

(event EventAddGameState
  (params (InState :type EGameState%20Enum :default "NewEnumerator0") (IsOtherRemove :type Boolean))
  (if IsOtherRemove
    (CallFunction|ResetGameState))
  (Utilities|Set|Add (Variables|Status|GetGameStateSet) InState))

(event EventAddGameStates
  (params (InStates :type Array%20of%20EGameState%20Enums :default "NewEnumerator0"))
  (Utilities|Set|AddItems (Variables|Status|GetGameStateSet) InStates))

(event EventRemoveGameStates
  (params (InStates :type Array%20of%20EGameState%20Enums :default "NewEnumerator0"))
  (Utilities|Set|RemoveItems (Variables|Status|GetGameStateSet) InStates))

(event EventResetGameState
  (Utilities|Set|Clear (Variables|Status|GetGameStateSet)))

(fn IsDebugMode
  (return (Variables|Status|GetIsDebug)))

(fn IsGameState
  (params (InState :type EGameState%20Enum :default "NewEnumerator0"))
  (return (Utilities|Set|Contains (Variables|Status|GetGameStateSet) InState)))

(fn IsGameStates
  (params (InStates :type Array%20of%20EGameState%20Enums :default "NewEnumerator0") (InCompareType :type ECompareType%20Enum :default "NewEnumerator0"))
  (switch Utilities|FlowControl|Switch|SwitchonECompareType InCompareType
    (:NewEnumerator0
      (LocalVariables|SetIsStateActive true)
      (for _array_element InStates
        (LocalVariables|SetIsStateActive (and (Utilities|Set|Contains (Variables|Status|GetGameStateSet) _array_element) (LocalVariables|GetIsStateActive)))))
    (:NewEnumerator1
      (for _array_element_2 InStates
        (LocalVariables|SetIsStateActive (or (Utilities|Set|Contains (Variables|Status|GetGameStateSet) _array_element_2) (LocalVariables|GetIsStateActive)))))
    (:NewEnumerator2
      (for _array_element_3 InStates
        (LocalVariables|SetIsStateActive (Class|KismetMathLibrary|XORBoolean (Utilities|Set|Contains (Variables|Status|GetGameStateSet) _array_element_3) false)))))
  (return (LocalVariables|GetIsStateActive)))

(fn RemoveGameState
  (params (InState :type EGameState%20Enum :default "NewEnumerator0"))
  (bind _returnvalue (Utilities|Set|Remove (Variables|Status|GetGameStateSet) InState))
  (return _returnvalue))
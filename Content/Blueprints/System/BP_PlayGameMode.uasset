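; Game mode for a local multiplayer fish game: it creates players and HUD/result widgets, starts the countdown, and matches player starts by tag.
; StartGamePlay sets the game state, timer and music.
; During play, Tick spawns AI enemy ships at random stage points from a timed DataTable, switches BGM after a set time, and calls Debug, which pushes player statuses to the result screen.
; Result ends play; RestartGame reloads StartMap.
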(event EventTick
  (params (DeltaSeconds :type Float%20%28single-precision%29))
  (bind _outsoundmanager (CallFunction|GetSoundManager))
  (bind _output_get (Variables|System|SetCurrentTime (- (Math|DateTime|Now) (Variables|System|GetStartTime))))
  (bind _isactive (Class|BPGameInstanceInterface|IsGameState(Message) (Game|GetGameInstance) "NewEnumerator2"))
  (if _isactive
    (Utilities|FlowControl|Sequence
      (:then_0
        (CallFunction|AddShipEvent)
        (CallFunction|Debug))
      (:then_1
        (if (>= (Math|Timespan|GetTotalSeconds _output_get) (Math|Conversions|ToFloat(Integer) (Utilities|String|ToString(Text) (Utilities|Text|FormatText "ゲームサウンドの変更時間"))))
          (Utilities|FlowControl|DoOnce false
            (:Completed
              (Default|StopBGM _outsoundmanager -1.0)
              (Default|PlayBackGroundMusic _outsoundmanager true "NewEnumerator2"))))))))

(event EventBeginPlay
  (CallFunction|Init))

(event EventStartGamePlay
  (Class|BPGameInstanceInterface|AddGameState(Message) (Game|GetGameInstance) "NewEnumerator2" true)
  (bind _returnvalue (Class|GameModeBase|GetNumPlayers))
  (for _index (range 0 _returnvalue)
    (Utilities|IsValid (Game|GetPlayerController _index)
      (:Is%20Valid
        (Class|BPPlayerInterface|StartPlayer(Message) (Game|GetPlayerController _index)))))
  (Variables|System|SetStartTime (Math|DateTime|Now))
  (Variables|System|SetCurrentTime (- (Math|DateTime|Now) (Variables|System|GetStartTime)))
  (Variables|/Game/Blueprints/Widget/BP_GameHUDWidget.BP_GameHUDWidget_C|SetIsGamePlay (Variables|System|GetGameHUDWidget) true)
  (Default|PlayBackGroundMusic (CallFunction|GetSoundManager) true "NewEnumerator3"))

(event EventRestartGame
  (bind _returnvalue (Game|GetCurrentLevelName true))
  (Game|OpenLevel(byName) "StartMap")
  (bind _returnvalue_2 (Class|GameModeBase|GetNumPlayers))
  (for _index (range 1 _returnvalue_2)
    (Class|GameplayStatics|RemovePlayer (Game|GetPlayerController _index) true)))

(fn ConstructionScript
  (bind _result (Utilities|Text|FormatText "ステージの半径"))
  (bind _returnvalue (Utilities|String|ToString(Text) _result))
  (bind _returnvalue_2 (Math|Conversions|ToFloat(Integer) _returnvalue))
  (Variables|Setting|SetStageSize (Math|Vector|MakeVector _returnvalue_2 _returnvalue_2 (Math|Conversions|ToFloat(Integer) (Utilities|String|ToString(Text) (Utilities|Text|FormatText "ステージの高さ"))))))

(fn Init
  (Utilities|FlowControl|Sequence
    (:then_0
      (Class|BPGameInstanceInterface|AddGameState(Message) (Game|GetGameInstance) "NewEnumerator9" true)
      (bind _returnvalue (UserInterface|CreateWidget "/Game/Blueprints/Widget/BP_GameHUDWidget.BP_GameHUDWidget_C"))
      (bind _output_get (Variables|System|SetGameHUDWidget _returnvalue))
      (UserInterface|Viewport|AddtoViewport _output_get 0)
      (bind _returnvalue_2 (UserInterface|CreateWidget "/Game/Blueprints/Widget/BP_ResultWidget.BP_ResultWidget_C"))
      (bind _output_get_2 (Variables|System|SetResultWidget _returnvalue_2))
      (UserInterface|Viewport|AddtoViewport _output_get_2 0))
    (:then_1
      (for _index (range 1 (- (Variables|Setting|GetPlayerCount) 1))
        (Class|GameplayStatics|CreatePlayer -1)
        (Default|Init (.AsBP%20Player%20Fish%20Character (Utilities|Casting|CastToBP_PlayerFishCharacter (Game|GetPlayerCharacter _index)))))
      (CallFunction|Startup))))

(fn Startup
  (for _index (range 0 (Variables|Setting|GetPlayerCount))
    (bind _asbp_miso_player_controller (Utilities|Casting|CastToBP_MisoPlayerController (Game|GetPlayerController _index)))
    (Default|ReadytoPlay _asbp_miso_player_controller))
  (Default|StartCountDown (Variables|System|GetGameHUDWidget)))

(fn ChoosePlayerStart
  (params (Player :type Controller%20Object%20Reference))
  (bind _outactors (Actor|GetAllActorsOfClass "/Script/Engine.PlayerStart"))
  (for _array_element _outactors
    (if (Utilities|Name|Equal(Name) (Variables|/Script/Engine.PlayerStart|GetPlayerStartTag _array_element) (Utilities|String|StringToName (Utilities|String|Right (Utilities|GetObjectName Player) 1)))
      (return _array_element))))

(fn Result
  (Class|BPGameInstanceInterface|AddGameState(Message) (Game|GetGameInstance) "NewEnumerator8" true)
  (for _index (range 0 (Variables|Setting|GetPlayerCount))
    (Class|BPPlayerInterface|GameEnd(Message) (Game|Player|GetPlayerPawn _index))
    (bind _outplayerstatus (Class|BPPlayerInterface|GetPlayerStatus(Message) (Game|Player|GetPlayerPawn _index)))
    (Utilities|Array|Add (LocalVariables|GetAllPlayerStatus) _outplayerstatus))
  (Default|StartResult (Variables|System|GetResultWidget) (LocalVariables|GetAllPlayerStatus)))

(fn Debug
  (for _index (range 0 (Variables|Setting|GetPlayerCount))
    (bind _outplayerstatus (Class|BPPlayerInterface|GetPlayerStatus(Message) (Game|Player|GetPlayerPawn _index)))
    (Utilities|Array|Add (LocalVariables|GetAllPlayerStatus) _outplayerstatus))
  (Default|StartResult (Variables|System|GetResultWidget) (LocalVariables|GetAllPlayerStatus)))

(fn AddShipEvent
  (bind _stagesize (Variables|Setting|GetStageSize))
  (bind _returnvalue (Math|Random|RandomPointinBoundingBox "0, 0, 0" _stagesize))
  (bind _returnvalue_2 (Utilities|GetDataTableRow "/Game/Blueprints/Data/AddShipEventTable.AddShipEventTable" (Utilities|String|StringToName (Utilities|String|ToString(Integer) (Variables|Event|GetCurrentAddShipEventCount))))
    (:then
      (bind _currenttime (CallFunction|GetCurrentTime))
      (if (>= (Math|Timespan|GetTotalSeconds _currenttime) (.ExecEventTime (Utilities|Struct|BreakStructAddShipEvent _returnvalue_2)))
        (for _index (range 0 (- (.AddShipCount (Utilities|Struct|BreakStructAddShipEvent _returnvalue_2)) 1))
          (bind _returnvalue_3 (AI|SpawnAIFromClass "/Game/Blueprints/Pawn/BP_EnemyShip.BP_EnemyShip_C" 0 (Math|Vector|MakeVector (.x _returnvalue) (.y _returnvalue) 5.7e+02) "0, 0, 0" false))
          (Default|SetupAI (.AsBP%20Enemy%20Ship (Utilities|Casting|CastToBP_EnemyShip _returnvalue_3)))
          (Variables|Event|SetCurrentAddShipEventCount (+ (Variables|Event|GetCurrentAddShipEventCount) 1)))))))

(fn GetCurrentTime
  (return (Variables|System|GetCurrentTime)))

(fn GetStageSize
  (return (Variables|Setting|GetStageSize)))
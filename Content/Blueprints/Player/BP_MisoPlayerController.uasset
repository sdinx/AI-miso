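; Player controller for the Miso player that keeps a set of active player states.
; Interface events add or remove states singly or in batches, and queries test one state or several with AND, OR or XOR.
; The XOR branch only reflects the last state checked, rather than a true exclusive-or.
; Init, SetPlayer and construction are empty, GetFishCount is a stub returning zero, and GetPlayerID returns the controller ID.
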(event EventBeginPlay
  (CallFunction|Init))

(event EventAddPlayerState
  (params (InState :type EPlayerState%20Enum :default "NewEnumerator0"))
  (Utilities|Set|Add (Variables|Status|GetPlayerStateSet) InState))

(event EventAddPlayerStates
  (params (InStates :type Array%20of%20EPlayerState%20Enums :default "NewEnumerator0"))
  (Utilities|Set|AddItems (Variables|Status|GetPlayerStateSet) InStates))

(event EventRemovePlayerStates
  (params (InStates :type Array%20of%20EPlayerState%20Enums :default "NewEnumerator0"))
  (Utilities|Set|RemoveItems (Variables|Status|GetPlayerStateSet) InStates))

(fn ConstructionScript)

(fn Init)

(fn SetPlayer)

(fn GetFishCount
  (return 0))

(fn GetPlayerID
  (return (Class|GameplayStatics|GetPlayerControllerID self)))

(fn IsPlayerState
  (params (InState :type EPlayerState%20Enum :default "NewEnumerator0"))
  (return (Utilities|Set|Contains (Variables|Status|GetPlayerStateSet) InState)))

(fn IsPlayerStates
  (params (InStates :type Array%20of%20EPlayerState%20Enums :default "NewEnumerator0") (InCompareType :type ECompareType%20Enum :default "NewEnumerator0"))
  (switch Utilities|FlowControl|Switch|SwitchonECompareType InCompareType
    (:NewEnumerator0
      (LocalVariables|SetIsStateActive true)
      (for _array_element InStates
        (LocalVariables|SetIsStateActive (and (Utilities|Set|Contains (Variables|Status|GetPlayerStateSet) _array_element) (LocalVariables|GetIsStateActive)))))
    (:NewEnumerator1
      (for _array_element_2 InStates
        (LocalVariables|SetIsStateActive (or (Utilities|Set|Contains (Variables|Status|GetPlayerStateSet) _array_element_2) (LocalVariables|GetIsStateActive)))))
    (:NewEnumerator2
      (for _array_element_3 InStates
        (LocalVariables|SetIsStateActive (Class|KismetMathLibrary|XORBoolean (Utilities|Set|Contains (Variables|Status|GetPlayerStateSet) _array_element_3) false)))))
  (return (LocalVariables|GetIsStateActive)))

(fn RemovePlayerState
  (params (InState :type EPlayerState%20Enum :default "NewEnumerator0"))
  (bind _returnvalue (Utilities|Set|Remove (Variables|Status|GetPlayerStateSet) InState))
  (return _returnvalue))
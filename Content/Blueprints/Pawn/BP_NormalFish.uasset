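; BP_NormalFish is an AI fish pawn that follows players, who can steal it from one another, updating their fish counts.
; It loads type, score and follow distance from a data table and runs a behavior tree, passing owner and target through blackboard keys.
; Movement smoothly rotates with clamped tilt.
; A new follow starts a countdown granting protection and extra speed, while Tick also toggles collision and retargets to player clones.
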(event EventBeginPlay
  (CallFunction|Init))

(event EventTick
  (params (DeltaSeconds :type Float%20%28single-precision%29))
  (bind _collisioncomponent (Variables|Default|GetCollisionComponent))
  (bind _followingplayerindex (Variables|Status|GetFollowingPlayerIndex))
  (bind _initspeed (Variables|Default|GetInitSpeed))
  (bind _returnvalue (Game|Player|GetPlayerPawn _followingplayerindex))
  (Utilities|FlowControl|Sequence
    (:then_0
      (bind _output_get (Variables|Default|SetDisableCollisionTime (+ DeltaSeconds (Variables|Default|GetDisableCollisionTime))))
      (if (>= _output_get 5.0)
        (switch Utilities|FlowControl|Switch|SwitchonECollisionEnabled (Collision|GetCollisionEnabled _collisioncomponent)
          (:NoCollision
            (Collision|SetCollisionEnabled _collisioncomponent "QueryAndPhysics"))
          (:QueryAndPhysics
            (Collision|SetCollisionEnabled _collisioncomponent "NoCollision")))))
    (:then_1
      (Utilities|IsValid _returnvalue
        (:Is%20Valid
          (bind (_isclone _clonefish) (Class|BPPlayerInterface|SplitFish(Message) _returnvalue))
          (if _isclone
            (Utilities|InputFollowingto _clonefish)))))
    (:then_2
      (bind _output_get_2 (Variables|Default|SetBreakDanceTime (- (Variables|Default|GetBreakDanceTime) 0.1)))
      (if (> _output_get_2 0.0)
        (Variables|Status|SetFMoveSpeed (+ _initspeed 0.5))
        (else
          (Variables|Status|SetFMoveSpeed _initspeed))))))

(event EventAddMovementInputOriginal
  (params (WorldDirection :type Vector :default "0, 0, 0") (ScaleValue :type Float%20%28single-precision%29))
  (bind _returnvalue (* WorldDirection -1.0))
  (bind _returnvalue_2 (Math|Rotator|MakeRotfromZ _returnvalue))
  (bind (_roll _pitch _yaw) (Math|Rotator|BreakRotator (Math|Rotator|MakeRotator 0.0 (.pitch _returnvalue_2) (.yaw _returnvalue_2))))
  ;[0 0 0] 移動処理
  (if (Variables|Status|GetIsFollowing)
    (Transformation|SetActorRotation (Math|Interpolation|RInterpTo (Transformation|GetActorRotation) (Math|Rotator|MakeRotator (Math|Float|Clamp(Float) _roll -3e+01 3e+01) (Math|Float|Clamp(Float) _pitch -3e+01 3e+01) _yaw) (Utilities|Time|GetWorldDeltaSeconds) 5.0))
    (if (Utilities|IsFollowDistance)
      (Pawn|Input|AddMovementInput WorldDirection (* (Variables|Status|GetFMoveSpeed) ScaleValue) false))))

(event EventSetParentPlayerIndex
  (params (InPlayerIndex :type Integer))
  (bind _blackboard (Variables|Default|GetBlackboard))
  (bind _output_get (Variables|Status|SetFollowingPlayerIndex InPlayerIndex))
  (Utilities|IsValid _blackboard
    (:Is%20Valid
      (Class|BlackboardComponent|SetValueasInt _blackboard (Utilities|String|StringToName "ParentPlayerIndex") _output_get))))

(event EventStartFollowing
  (params (InPlayerIndex :type Integer) (InFollowingType :type EFollowingType%20Enum :default "NewEnumerator0") (InPawn :type Pawn%20Object%20Reference))
  (bind _followingplayerindex (Variables|Status|GetFollowingPlayerIndex))
  (if (!= InPlayerIndex _followingplayerindex)
    (if (== _followingplayerindex -1)
      _
      (else
        (Class|BPPlayerInterface|SubFish(Message) (Game|GetPlayerController (Variables|Status|GetFollowingPlayerIndex)) (Variables|Const|GetFishType))
        (Class|BPPlayerInterface|SubLocalFishCount(Message) InPawn)))
    (CallFunction|SetParentPlayerIndex InPlayerIndex)
    (Utilities|InputFollowingto InPawn)
    (Class|BPPlayerInterface|AddFish(Message) (Game|GetPlayerController InPlayerIndex) (Variables|Const|GetFishType))
    (Variables|Status|SetIsFollowing true)
    (Class|BPPlayerInterface|AddLocalFishCount(Message) InPawn)
    (Variables|Default|SetBreakDanceTime 1e+01)))

(event EventSetProtectFish
  (params (IsActive :type Boolean))
  (Variables|Default|SetIsProtected IsActive))

(event EventCapturedFish
  (bind _followingplayerindex (Variables|Status|GetFollowingPlayerIndex))
  (bind _returnvalue (Game|Player|GetPlayerPawn _followingplayerindex))
  (Actor|DestroyActor)
  (Utilities|IsValid _returnvalue
    (:Is%20Valid
      (Class|BPPlayerInterface|SubFish(Message) _returnvalue (Variables|Const|GetFishType)))))

(fn ConstructionScript)

(fn Init
  (bind _meshcomponent (Variables|GetMeshComponent))
  (bind _isdebug (Class|BPGameInstanceInterface|IsDebugMode(Message) (Game|GetGameInstance)))
  (if _isdebug
    (CallFunction|SetupDebugOnly))
  (Private|SetupFishStatus)
  (Variables|Status|SetFollowingPlayerIndex -1)
  (Utilities|IsValid _meshcomponent
    (:Is%20Valid
      (Components|DestroyComponent _meshcomponent))
    (:Is%20Not%20Valid
      _))
  (CallFunction|SetupAI)
  (Variables|/Script/Engine.SkinnedMeshComponent|SetVisibilityBasedAnimTickOption (Variables|Default|GetSkeletalMesh) "OnlyTickPoseWhenRendered")
  (Variables|Default|SetInitSpeed (Variables|Status|GetFMoveSpeed)))

(fn SetupDebugOnly
  (Development|SetHiddeninGame (Variables|Default|GetCollisionComponent) false false))

(fn SetupAI
  (bind _asaicontroller (Utilities|Casting|CastToAIController (Pawn|GetController)))
  (bind _blackboardcomponent (Class|AIController|UseBlackboard _asaicontroller "/Game/Blueprints/AI/BB_Fish.BB_Fish"))
  (Variables|Default|SetBlackboard _blackboardcomponent)
  (bind _returnvalue (AI|RunBehaviorTree _asaicontroller (Variables|Default|GetRunBehavior)))
  (Variables|Status|SetIsFollowing _returnvalue)
  (CallFunction|SetParentPlayerIndex -1))

(fn SetupFishStatus
  (bind _returnvalue (Utilities|GetDataTableRow "/Game/Blueprints/Data/FishStatusTable.FishStatusTable" (Variables|Const|GetFishName))
    (:then
      (Variables|Const|SetFishType (.fishtype _returnvalue))
      (Variables|Const|SetFScorePoint (.fscorepoint _returnvalue))
      (Variables|Const|SetFDistanceToFollow (.fdistancetofollow _returnvalue)))))

(fn SetSpawnAreaActor
  (params (InLocation :type BP%20Fish%20Spawn%20Point%20Object%20Reference))
  (AI|Components|Blackboard|SetValueasObject (Variables|Default|GetBlackboard) (Utilities|String|StringToName "SpawnAreaActor") InLocation))

(fn GetParentPlayerIndex
  (return (Variables|Status|GetFollowingPlayerIndex)))

(fn GetScorePoint
  (return (Variables|Const|GetFScorePoint)))

(fn IsProtect
  (if (Variables|Default|GetIsProtected)
    (return true)
    (else
      (return (> (Variables|Default|GetBreakDanceTime) 0.0)))))
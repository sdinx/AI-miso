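; BP_CloneFish is an AI-driven fish pawn, tagged with a parent player index, that recruits other fish to follow it.
; On BeginPlay it starts a behavior tree on the BB_Fish blackboard.
; Its LearnRadius sphere makes unprotected overlapping actors follow it and marks them protected, clearing that on exit if the player index matches.
; Movement input also smoothly turns the fish toward its heading with clamped pitch.
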(event EventBeginPlay
  (CallFunction|Init))

(event EventSetParentPlayerIndex
  (params (InPlayerIndex :type Integer))
  (Variables|Status|SetnPlayerIndex InPlayerIndex))

(event EventAddMovementInputOriginal
  (params (WorldDirection :type Vector :default "0, 0, 0") (ScaleValue :type Float%20%28single-precision%29))
  (bind _returnvalue (* WorldDirection 1.0))
  (bind _returnvalue_2 (Math|Rotator|MakeRotfromX _returnvalue))
  (bind (_roll _pitch _yaw) (Math|Rotator|BreakRotator (Math|Rotator|MakeRotator 0.0 (.pitch _returnvalue_2) (.yaw _returnvalue_2))))
  ;[0 0 0] 移動処理
  (Transformation|SetActorRotation (Math|Interpolation|RInterpTo (Transformation|GetActorRotation) (Math|Rotator|MakeRotator (Math|Float|Clamp(Float) _roll -3e+01 3e+01) (Math|Float|Clamp(Float) _pitch -3e+01 3e+01) _yaw) (Utilities|Time|GetWorldDeltaSeconds) 5.0))
  (Pawn|Input|AddMovementInput WorldDirection (* 1.0 ScaleValue) false))

(event OnComponentBeginOverlap(CollisionComponent)
  (params (OverlappedComponent :type Primitive%20Component%20Object%20Reference) (OtherActor :type Actor%20Object%20Reference) (OtherComp :type Primitive%20Component%20Object%20Reference) (OtherBodyIndex :type Integer) (bFromSweep :type Boolean) (SweepResult :type Hit%20Result%20Structure%20%28by%20ref%29))
  (bind _isactive (Class|BPFishInterface|IsProtect(Message) OtherActor))
  (if (not _isactive)
    (Class|BPFishInterface|StartFollowing(Message) OtherActor (Variables|Status|GetnPlayerIndex) "NewEnumerator1" self)
    (Class|BPFishInterface|SetProtectFish(Message) OtherActor true)))

(event OnComponentEndOverlap(CollisionComponent)
  (params (OverlappedComponent :type Primitive%20Component%20Object%20Reference) (OtherActor :type Actor%20Object%20Reference) (OtherComp :type Primitive%20Component%20Object%20Reference) (OtherBodyIndex :type Integer))
  (bind _outplayerindex (Class|BPFishInterface|GetParentPlayerIndex(Message) OtherActor))
  (if (== _outplayerindex (Variables|Status|GetnPlayerIndex))
    (Class|BPFishInterface|SetProtectFish(Message) OtherActor false)))

(fn ConstructionScript
  (Components|Sphere|SetSphereRadius (Variables|Default|GetCollisionComponent) (Variables|Status|GetLearnRadius) true))

(fn Init
  (CallFunction|SetupAI))

(fn SetupAI
  (bind _asaicontroller (Utilities|Casting|CastToAIController (Pawn|GetController)))
  (bind _blackboardcomponent (Class|AIController|UseBlackboard _asaicontroller "/Game/Blueprints/AI/BB_Fish.BB_Fish"))
  (Variables|Default|SetBlackboard _blackboardcomponent)
  (AI|RunBehaviorTree _asaicontroller (Variables|Default|GetRunBehavior)))

(fn SetLearnRadius
  (params (InRadius :type Float%20%28single-precision%29))
  (bind _output_get (Variables|Status|SetLearnRadius 0.0))
  (Class|BPPlayerInterface|UpdateLearnRadius(Message) (Variables|Default|GetCollisionComponent) _output_get))

(fn GetParentPlayerIndex
  (return (Variables|Status|GetnPlayerIndex)))

(fn IsProtect
  (return false))
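; BP_EnemyShip is an AI-driven enemy ship pawn with a net that sends a captured-fish message to actors it hits.
; BeginPlay starts its behavior tree and blackboard.
; During one game state, Tick steps through a DataTable of timed events, rescaling the net pivot as game-mode time reaches each row.
; A custom movement event smoothly turns the ship toward its direction, clamping pitch and roll, and adds speed-scaled input.
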(event OnComponentBeginOverlap(CaptureNet)
  (params (OverlappedComponent :type Primitive%20Component%20Object%20Reference) (OtherActor :type Actor%20Object%20Reference) (OtherComp :type Primitive%20Component%20Object%20Reference) (OtherBodyIndex :type Integer) (bFromSweep :type Boolean) (SweepResult :type Hit%20Result%20Structure%20%28by%20ref%29)))

(event OnComponentHit(CaptureNet)
  (params (HitComponent :type Primitive%20Component%20Object%20Reference) (OtherActor :type Actor%20Object%20Reference) (OtherComp :type Primitive%20Component%20Object%20Reference) (NormalImpulse :type Vector :default "0, 0, 0") (Hit :type Hit%20Result%20Structure%20%28by%20ref%29))
  (Class|BPFishInterface|CapturedFish(Message) OtherActor))

(event EventBeginPlay
  (CallFunction|SetupAI))

(event Collision|EventActorBeginOverlap
  (params (OtherActor :type Actor%20Object%20Reference)))

(event EventTick
  (params (DeltaSeconds :type Float%20%28single-precision%29))
  (bind _isactive (Class|BPGameInstanceInterface|IsGameState(Message) (Game|GetGameInstance) "NewEnumerator2"))
  (if _isactive
    (CallFunction|TimerEvent)))

(event EventAddMovementInputCustom
  (params (WorldDirection :type Vector :default "0, 0, 0") (ScaleValue :type Float%20%28single-precision%29))
  (bind _returnvalue (* WorldDirection 1.0))
  (bind _returnvalue_2 (Math|Rotator|MakeRotfromX _returnvalue))
  (bind (_roll _pitch _yaw) (Math|Rotator|BreakRotator (Math|Rotator|MakeRotator 0.0 (.pitch _returnvalue_2) (.yaw _returnvalue_2))))
  ;[0 0 0] 移動処理
  (Transformation|SetActorRotation (Math|Interpolation|RInterpTo (Transformation|GetActorRotation) (Math|Rotator|MakeRotator (Math|Float|Clamp(Float) _roll -3e+01 3e+01) (Math|Float|Clamp(Float) _pitch -3e+01 3e+01) _yaw) (Utilities|Time|GetWorldDeltaSeconds) 5.0))
  (Pawn|Input|AddMovementInput WorldDirection (* (Variables|Default|GetMoveSpeed) ScaleValue) false))

(fn ConstructionScript)

(fn SetupAI
  (bind _asaicontroller (Utilities|Casting|CastToAIController (Pawn|GetController)))
  (bind _blackboardcomponent (Class|AIController|UseBlackboard _asaicontroller "/Game/Blueprints/AI/BB_EnemyShip.BB_EnemyShip"))
  (Variables|Default|SetBlackboard _blackboardcomponent)
  (AI|RunBehaviorTree _asaicontroller (Variables|Default|GetRunBehavior)))

(fn TimerEvent
  (bind _returnvalue (Utilities|GetDataTableRow "/Game/Blueprints/Data/EnemyShipEventTable.EnemyShipEventTable" (Utilities|String|StringToName (Utilities|String|ToString(Integer) (Variables|Default|GetCurrentEventCount))))
    (:then
      (bind _currenttime (Class|BPPlayModeInterface|GetCurrentTime(Message) (Game|GetGameMode)))
      (if (>= (Math|Timespan|GetTotalSeconds _currenttime) (.ExecEventTime (Utilities|Struct|BreakStructEnemyShipEvent _returnvalue)))
        (Variables|Default|SetCurrentEventCount (+ (Variables|Default|GetCurrentEventCount) 1))
        (Transformation|SetWorldScale3D (Variables|Default|GetCaptureNetPivot) (Math|Conversions|ToVector(Float) (.CaptureNetScale (Utilities|Struct|BreakStructEnemyShipEvent _returnvalue))))))))
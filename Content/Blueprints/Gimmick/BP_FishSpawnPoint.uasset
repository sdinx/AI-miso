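; Fish spawn point that periodically spawns batches of AI fish around a visible spawn-area component, which shows in game only in debug mode.
; The construction script loads timing, count, extents and fish class from a data table row keyed by FishType and scales the area to match.
; While the game instance reports the required state, Tick counts down to randomized batches.
; Each batch shares one random location, and each fish receives this actor as its spawn area.
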(event EventBeginPlay
  (CallFunction|Init))

(event EventTick
  (params (DeltaSeconds :type Float%20%28single-precision%29))
  (bind _spawntimerandomrange (Variables|Status|GetSpawnTimeRandomRange))
  (bind _spawncountrandomrange (Variables|Status|GetSpawnCountRandomRange))
  (bind _isactive (Class|BPGameInstanceInterface|IsGameState(Message) (Game|GetGameInstance) "NewEnumerator2"))
  (if _isactive
    (bind _output_get (Variables|Status|SetCurrentTime (- (Variables|Status|GetCurrentTime) DeltaSeconds)))
    (if (<= _output_get 0.0)
      (Variables|Status|SetCurrentTime (+ (Variables|Status|GetSpawnTime) (Math|Random|RandomFloatinRange (* _spawntimerandomrange -1.0) _spawntimerandomrange)))
      (CallFunction|SpawnFish (+ (Variables|Status|GetSpawnCount) (Math|Random|RandomIntegerinRange (* _spawncountrandomrange -1) _spawncountrandomrange))))))

(fn ConstructionScript
  (bind _returnvalue (Utilities|GetDataTableRow "/Game/Blueprints/Data/SpawnFishInfoTable.SpawnFishInfoTable" (Utilities|String|StringToName (Utilities|String|EnumtoString (Variables|Setting|GetFishType))))
    (:then
      (Variables|Status|SetCurrentTime (.FirstDelaySpawnTime (Utilities|Struct|BreakStructSpawnInfo _returnvalue)))
      ;[0 0 0] 魚のスポーン情報の取得
      (Variables|Status|SetSpawnTime (.SpawnTime (Utilities|Struct|BreakStructSpawnInfo _returnvalue)))
      (Variables|Status|SetSpawnTimeRandomRange (.SpawnTimeRandomRange (Utilities|Struct|BreakStructSpawnInfo _returnvalue)))
      (Variables|Status|SetSpawnCount (.SpawnCount (Utilities|Struct|BreakStructSpawnInfo _returnvalue)))
      (Variables|Status|SetSpawnCountRandomRange (.SpawnCountRandomRange (Utilities|Struct|BreakStructSpawnInfo _returnvalue)))
      (LocalVariables|SetSpawnRadius (.SpawnRadius (Utilities|Struct|BreakStructSpawnInfo _returnvalue)))
      (LocalVariables|SetSpawnHalfHeight (.SpawnHalfHeight (Utilities|Struct|BreakStructSpawnInfo _returnvalue)))
      (Variables|Status|SetSpawnFishClass (.SpawnFishClass (Utilities|Struct|BreakStructSpawnInfo _returnvalue)))
      (Transformation|SetWorldScale3D (Variables|Default|GetVisibleSpawnArea) (Math|Vector|MakeVector (* (LocalVariables|GetSpawnRadius) 2.0 0.01) (* (LocalVariables|GetSpawnRadius) 2.0 0.01) (* (LocalVariables|GetSpawnHalfHeight) 2.0 0.01))))))

(fn SpawnFish
  (params (InFishCount :type Integer))
  (bind _outspawnlocation (CallFunction|GetRandomSpawnLocation))
  (LocalVariables|SetSpawnLocation _outspawnlocation)
  (for _index (range 0 InFishCount)
    (bind _returnvalue (AI|SpawnAIFromClass (Variables|Status|GetSpawnFishClass) 0 (LocalVariables|GetSpawnLocation) "0, 0, 0" false))
    (bind _asbp_normal_fish (Utilities|Casting|CastToBP_NormalFish _returnvalue))
    (Default|Init _asbp_normal_fish)
    (Default|SetSpawnAreaActor _asbp_normal_fish self)))

(fn GetRandomSpawnLocation
  (bind (_radius _halfheight) (Utilities|GetSpawnRadiusandHalfHeight))
  (bind _visiblespawnarea (Variables|Default|GetVisibleSpawnArea))
  (bind _returnvalue (Transformation|GetWorldLocation _visiblespawnarea))
  (bind _returnvalue_2 (* _radius -1.0))
  (return (Math|Vector|MakeVector (+ (Math|Random|RandomFloatinRange _returnvalue_2 _radius) (.x _returnvalue)) (+ (Math|Random|RandomFloatinRange _returnvalue_2 _radius) (.y _returnvalue)) (+ (.z _returnvalue) (Math|Random|RandomFloatinRange 0.0 _halfheight)))))

(fn Init
  (bind _visiblespawnarea (Variables|Default|GetVisibleSpawnArea))
  (bind _isdebug (Class|BPGameInstanceInterface|IsDebugMode(Message) (Game|GetGameInstance)))
  (if _isdebug
    (Rendering|SetVisibility _visiblespawnarea true false)
    (Development|SetHiddeninGame _visiblespawnarea false false)
    (else
      (Rendering|SetVisibility _visiblespawnarea false false)
      (Development|SetHiddeninGame _visiblespawnarea true false))))
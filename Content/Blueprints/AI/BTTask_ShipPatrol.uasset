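; Behavior tree task that makes an AI ship patrol back and forth along the X axis of the stage.
; On its first tick it gets the stage size from the game mode and derives a patrol range slightly inside the X size.
; Each tick flips the target X when the pawn is at or beyond either limit, writes FlyToLocation with current Y and Z to the blackboard, and finishes successfully.
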(event EventReceiveTickAI
  (params (OwnerController :type AI%20Controller%20Object%20Reference) (ControlledPawn :type Pawn%20Object%20Reference) (DeltaSeconds :type Float%20%28single-precision%29))
  (bind _returnvalue (Transformation|GetActorLocation ControlledPawn))
  (bind (_x _y _z) (Math|Vector|BreakVector _returnvalue))
  (bind _x_2 (Math|Vector|BreakVector _returnvalue))
  (Utilities|FlowControl|Sequence
    (:then_0
      (Utilities|FlowControl|DoOnce false
        (:Completed
          (bind _outstagesize (Class|BPPlayModeInterface|GetStageSize(Message) (Game|GetGameMode)))
          (bind _output_get (Variables|Default|SetPatrolRange (/ (.X (Math|Vector|BreakVector _outstagesize)) 1.1)))
          (Variables|Default|SetCurrentPatrolXPos _output_get))))
    (:then_1
      (if (or (>= _x_2 (Variables|Default|GetPatrolRange)) (<= _x_2 (* (Variables|Default|GetPatrolRange) -1.0)))
        (Variables|Default|SetCurrentPatrolXPos (* (Variables|Default|GetCurrentPatrolXPos) -1.0))))
    (:then_2
      (AI|BehaviorTree|SetBlackboardValueasVector (Variables|Default|GetFlyToLocation) (Math|Vector|MakeVector (Variables|Default|GetCurrentPatrolXPos) _y _z))
      (AI|BehaviorTree|FinishExecute true))))
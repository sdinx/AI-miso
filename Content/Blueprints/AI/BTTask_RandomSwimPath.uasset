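; Behavior tree task that periodically picks random swim destinations for an AI within the stage bounds.
; Its AI tick accumulates time against MoveChangeTime and resets the timer when a new point is chosen.
; The point comes from a box centered on the world origin, sized by the game mode's GetStageSizeMessage, and is written to the FlyToLocationKey blackboard key.
; The task never calls Finish Execute.
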(event EventReceiveTickAI
  (params (OwnerController :type AI%20Controller%20Object%20Reference) (ControlledPawn :type Pawn%20Object%20Reference) (DeltaSeconds :type Float%20%28single-precision%29))
  (bind _output_get (Variables|Default|SetMoveTimer (+ DeltaSeconds (Variables|Default|GetMoveTimer))))
  (if (>= _output_get (Variables|Default|GetMoveChangeTime))
    _
    (else
      (Utilities|FlowControl|DoOnce false
        (:Completed
          _))))
  (Variables|Default|SetMoveTimer 0.0)
  (bind _outstagesize (Class|BPPlayModeInterface|GetStageSize(Message) (Game|GetGameMode)))
  (AI|BehaviorTree|SetBlackboardValueasVector (Variables|Default|GetFlyToLocationKey) (Math|Random|RandomPointinBoundingBox "0, 0, 0" _outstagesize)))
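; Behavior tree task that steers an AI pawn along a circling path by updating FlyToLocation every tick.
; On first tick it stores the pawn's location, derives a start yaw from SpawnAreaLocation and randomly picks a direction.
; Each tick it grows the angle using game mode time, rotates the stored world location and adds the area's XY.
; FinishExecute is unconnected, so the task never completes itself.
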(event EventReceiveTickAI
  (params (OwnerController :type AI%20Controller%20Object%20Reference) (ControlledPawn :type Pawn%20Object%20Reference) (DeltaSeconds :type Float%20%28single-precision%29))
  (Utilities|FlowControl|Sequence
    (:then_0
      (Utilities|FlowControl|DoOnce false
        (:Completed
          (CallFunction|Init (Transformation|GetActorLocation ControlledPawn) (Class|BTFunctionLibrary|GetBlackboardValueasVector (Variables|Default|GetSpawnAreaLocation))))))
    (:then_1
      (bind _outlocation (CallFunction|GetNextLocation (Class|BTFunctionLibrary|GetBlackboardValueasVector (Variables|Default|GetSpawnAreaLocation))))
      (AI|BehaviorTree|SetBlackboardValueasVector (Variables|Default|GetFlyToLocation) _outlocation))))

(fn GetNextLocation
  (params (InCenter :type Vector))
  (bind _currenttime (Class|BPPlayModeInterface|GetCurrentTime(Message) (Game|GetGameMode)))
  (bind _output_get (Variables|Default|SetAngle (+ (Variables|Default|GetAngle) (* (Math|Timespan|GetTotalSeconds _currenttime) (Variables|Default|GetAddAngle)))))
  (return (+ (Math|Vector|RotateVector (Variables|Default|GetCurrentLocation) (Math|Rotator|MakeRotator 0.0 0.0 _output_get)) (Math|Vector|MakeVector (.x InCenter) (.y InCenter) 0.0))))

(fn Init
  (params (Current :type Vector) (Center :type Vector))
  (bind (_x _y) (Math|Vector|BreakVector Center))
  (bind _output_get (Variables|Default|SetCurrentLocation Current))
  (Variables|Default|SetAngle (.yaw (Math|Rotator|FindLookatRotation (Math|Vector|MakeVector _x _y 0.0) (Math|Vector|MakeVector (.X (Math|Vector|BreakVector _output_get)) (.Y (Math|Vector|BreakVector _output_get)) 0.0))))
  (if (Math|Random|RandomBool)
    (Variables|Default|SetAddAngle (* (Variables|Default|GetAddAngle) -1.0))))